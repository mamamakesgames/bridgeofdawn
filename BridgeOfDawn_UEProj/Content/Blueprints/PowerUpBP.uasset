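; PowerUpBP is a pickup that grants the player a timed stamina, jump, sprint or score-multiplier power-up.
; On BeginPlay it either destroys itself by spawn chance or keeps its type, picking one at random if None.
; The type sets an index on a dynamic texture-array material created in the construction script, selecting the icon on a plane that spins on Tick.
; Overlap by BOD_PlayerCharacter calls StartPowerUp with type and duration, then destroys the pickup.
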(event `self.ReceiveBeginPlay`
  (bind _icon_texarray_dynamic_material (`self.Icon TexArray Dynamic Material`))
  ;[0.9 0.3 1] Check if should "spawn" and set icon - KAB
  (if (<= (`KismetMathLibrary.RandomFloat`) (`self.Chance of Spawning`))
    (switch `/Game/Blueprints/BOD_PowerUpType` (`self.PowerUp Type`) :!label _label ; 0=Jump, 1=Sprint, 2=TopSpeed, 3=x2points, 4=x3points
      (:`NewEnumerator0`
        (switch `int` (`KismetMathLibrary.RandomIntegerInRange` 0 4)
          (:`Default`
            _)
          (:`0`
            _)
          (:`1`
            (set `self.PowerUp Type` "NewEnumerator2")
            (goto _label))
          (:`2`
            (set `self.PowerUp Type` "NewEnumerator3")
            (goto _label))
          (:`3`
            (set `self.PowerUp Type` "NewEnumerator4")
            (goto _label))
          (:`4`
            (set `self.PowerUp Type` "NewEnumerator5")
            (goto _label)))
        (set `self.PowerUp Type` "NewEnumerator1")
        (goto _label))
      (:`NewEnumerator1`
        (`MaterialInstanceDynamic.SetScalarParameterValue` _icon_texarray_dynamic_material "PowerUp Index" 1.0))
      (:`NewEnumerator2`
        (`MaterialInstanceDynamic.SetScalarParameterValue` _icon_texarray_dynamic_material "PowerUp Index" 0.0))
      (:`NewEnumerator3`
        (`MaterialInstanceDynamic.SetScalarParameterValue` _icon_texarray_dynamic_material "PowerUp Index" 2.0))
      (:`NewEnumerator4`
        (`MaterialInstanceDynamic.SetScalarParameterValue` _icon_texarray_dynamic_material "PowerUp Index" 3.0))
      (:`NewEnumerator5`
        (`MaterialInstanceDynamic.SetScalarParameterValue` _icon_texarray_dynamic_material "PowerUp Index" 4.0)))
    (else
      (`self.K2_DestroyActor`))))

(event `self.ReceiveTick`
  (params (DeltaSeconds :type "Float (single-precision)"))
  ;[0.9 0.3 1] Rotate with event tick - KAB
  (`SceneComponent.K2_AddRelativeRotation` (`self.Plane`) (`KismetMathLibrary.MakeRotator` 0.0 0.0 (`KismetMathLibrary.Lerp` 0.0 100.0 DeltaSeconds)) false true))

(event `self.ReceiveActorBeginOverlap`
  (params (OtherActor :type "Actor Object Reference"))
  ;[0.9 0.3 1] On touch by player, activate power up and remove self - KAB
  (bind _asbod_player_character (cast `/Game/Characters/BOD_PlayerCharacter` OtherActor))
  (`/Game/Characters/BOD_PlayerCharacter.Start PowerUp` _asbod_player_character (`self.PowerUp Type`) (`self.Effect Duration`))
  (`self.K2_DestroyActor`))

(fn `UserConstructionScript`
  ;[0.9 0.3 1] Create dynamic material for texture array icon - KAB
  (bind _returnvalue (`PrimitiveComponent.CreateDynamicMaterialInstance` (`self.Plane`) 0 null "None"))
  (set `self.Icon TexArray Dynamic Material` _returnvalue))