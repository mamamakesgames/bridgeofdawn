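; Waypoint pickup actor that its owning player character touches to score points and advance to the next waypoint.
; Tick spins the Waypoint component on roll and the Cone on yaw, scaled by delta time.
; When the capsule overlaps the owner, it calls SetNextWaypoint on BOD_PlayerCharacter, awards points equal to the rounded-up distance between them, then destroys itself.
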(event `self.ReceiveTick`
  (params (DeltaSeconds :type "Float (single-precision)"))
  ;[0.9 0.3 1] Rotate with event tick - KAB
  (`SceneComponent.K2_AddRelativeRotation` (`self.Waypoint`) (`KismetMathLibrary.MakeRotator` (`KismetMathLibrary.Lerp` 0.0 100.0 DeltaSeconds) 0.0) false false)
  (`SceneComponent.K2_AddRelativeRotation` (`self.Cone`) (`KismetMathLibrary.MakeRotator` 0.0 0.0 (`KismetMathLibrary.Lerp` 0.0 100.0 DeltaSeconds)) false false))

(event `self.Collision Capsule.OnComponentBeginOverlap`
  (params (OverlappedComponent :type "PrimitiveComponent Object Reference") (OtherActor :type "Actor Object Reference") (OtherComp :type "PrimitiveComponent Object Reference") (OtherBodyIndex :type Integer) (bFromSweep :type Boolean) (SweepResult :type "HitResult Structure (by ref)"))
  (bind _returnvalue (`self.GetOwner`))
  ;[0.9 0.3 1] When player touches waypoint, add points, and switch to next waypoint - KAB
  (if (== OtherActor _returnvalue)
    (bind _asbod_player_character (cast `/Game/Characters/BOD_PlayerCharacter` _returnvalue))
    (`/Game/Characters/BOD_PlayerCharacter.Set Next Waypoint` _asbod_player_character)
    (`/Game/Characters/BOD_PlayerCharacter.Add New Points To Score` _asbod_player_character (`KismetMathLibrary.FCeil` (`self.GetDistanceTo` _asbod_player_character self)) 1.0 (struct :`R` 1.0 :`G` 1.0 :`A` 1.0))
    (`self.K2_DestroyActor`)))

(fn `UserConstructionScript`)