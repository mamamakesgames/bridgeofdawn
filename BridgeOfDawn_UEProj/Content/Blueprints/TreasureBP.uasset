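; Treasure pickup actor that spins on Tick and awards points to the player character on overlap, then plays a sound and destroys itself.
; On BeginPlay it uses chance weights to either remove itself or keep one of three gem tiers, setting that tier's random point range and message color.
; Each tier check draws a fresh random number, so actual odds differ from the weights.
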(event `self.ReceiveBeginPlay`
  (`self.Select Correct Gem`))

(event `self.ReceiveTick`
  (params (DeltaSeconds :type "Float (single-precision)"))
  ;[0.9 0.3 1] Rotate with event tick - KAB
  (`self.K2_AddActorWorldRotation` (`KismetMathLibrary.MakeRotator` 0.0 0.0 (`KismetMathLibrary.Lerp` 0.0 100.0 DeltaSeconds)) false true))

(event `self.ReceiveActorBeginOverlap`
  (params (OtherActor :type "Actor Object Reference"))
  ;[0.9 0.3 1] On touch by player, give treasure and good feelings - KAB
  (bind _asbod_player_character (cast `/Game/Characters/BOD_PlayerCharacter` OtherActor))
  (`/Game/Characters/BOD_PlayerCharacter.Add New Points To Score` _asbod_player_character (`self.Points`) 1.0 (`self.Message Color`))
  (`GameplayStatics.PlaySound2D` "/Game/Audio/SoundEffects/treasure.treasure" 1.0 1.0 0.0 null null)
  (`self.K2_DestroyActor`))

(fn `Select Correct Gem`
  (bind _chance_of_nothing (`self.Chance of Nothing`))
  (bind _returnvalue (+ _chance_of_nothing (`self.Chance of Good`)))
  (bind _returnvalue_2 (* (`KismetMathLibrary.RandomFloat`) (+ (`self.Chance of Nothing`) (`self.Chance of Good`) (`self.Chance of Better`) (`self.Chance of Best`))))
  ;[0.9 0.3 1] Set points and color according to a randomized selection - KAB
  (if (< _returnvalue_2 _chance_of_nothing)
    (`self.K2_DestroyActor`)
    (elif (< _returnvalue_2 _returnvalue)
      (`ActorComponent.K2_DestroyComponent` (`self.BetterGem`))
      (`ActorComponent.K2_DestroyComponent` (`self.BestGem`))
      (set `self.Points` (`KismetMathLibrary.RandomIntegerInRange` 1 99))
      (set `self.Message Color` (struct :`G` 0.8 :`A` 1.0))
      (elif (< _returnvalue_2 (+ _returnvalue (`self.Chance of Better`)))
        (`ActorComponent.K2_DestroyComponent` (`self.GoodGem`))
        (`ActorComponent.K2_DestroyComponent` (`self.BestGem`))
        (set `self.Points` (`KismetMathLibrary.RandomIntegerInRange` 100 299))
        (set `self.Message Color` (struct :`R` 0.3 :`G` 0.3 :`B` 1.0 :`A` 1.0))
        (else
          (`KismetSystemLibrary.PrintString` "Hello")
          (`ActorComponent.K2_DestroyComponent` (`self.GoodGem`))
          (`ActorComponent.K2_DestroyComponent` (`self.BetterGem`))
          (set `self.Points` (`KismetMathLibrary.RandomIntegerInRange` 300 2000))
          (set `self.Message Color` (struct :`R` 1.0 :`A` 1.0)))))))

(fn `UserConstructionScript`)