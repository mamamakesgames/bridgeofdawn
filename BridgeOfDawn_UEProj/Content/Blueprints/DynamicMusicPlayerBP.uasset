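; Layered dynamic music player that starts all song stems together and mixes them by volume from a 0..1 gameplay progress value.
; A vector curve drives the foundation and two progress layers; AdvanceProgress only moves forward, for two-player mode.
; Registered tension actors toggle the tension layer, and Tick switches the boost layer using BoostUntil.
; Volumes change instantly, scaled by the game instance's music setting; ChangeToFinished fades out everything except the finished song.
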(event `self.ReceiveTick`
  (params (DeltaSeconds :type "Float (single-precision)"))
  (bind _boost_song_handle (`self.Boost Song Handle`))
  (bind _returnvalue (== (`AudioComponent.VolumeMultiplier` _boost_song_handle) 1.0))
  ;[0.9 0.3 1] Adjust boost if needed - KAB
  (bind _adjustable (`self.Is Adjustable?`))
  (if _adjustable
    (if (> (`self.Boost Until`) (`KismetSystemLibrary.GetGameTimeInSeconds`))
      (if (not _returnvalue)
        (`AudioComponent.SetVolumeMultiplier` _boost_song_handle (`self.Master Volume Adjustment`)))
      (elif _returnvalue
        (`AudioComponent.SetVolumeMultiplier` _boost_song_handle (`self.Minimum Volume Level`))))))

(fn `Advance Progress`
  (params (Progress :type "Float (double-precision)"))
  ;[0.9 0.3 1] This only calls Update Progress if it is increasing. Important for two-player mode - KAB
  (if (> Progress (`self.Last Progress`))
    (`self.Update Progress` Progress)))

(fn `Change to Finished`
  ;[0.9 0.3 1] Stop all other songs and switch to Finished Song - KAB
  (bind _adjustable (`self.Is Adjustable?`))
  (if _adjustable
    (for _array_element (`self.Song Handle Basket`)
      (if (!= (`self.Finished Song Handle`) _array_element)
        (`self.Remove Song Handle` _array_element)))
    (`AudioComponent.SetVolumeMultiplier` (`self.Finished Song Handle`) (`self.Master Volume Adjustment`))))

(fn `Clear All Tension`
  (locals (`Should Update` :type Boolean))
  ;[0.9 0.3 1] Remove all tensions and, if changed, update audio using last progress - KAB
  (if (> (`BlueprintSetLibrary.Set_Length` (`self.Tension Actors`)) 0)
    (`BlueprintSetLibrary.Set_Clear` (`self.Tension Actors`))
    (`self.Update Progress` (`self.Last Progress`))))

(fn `Faded Adjustment`
  (params (Song :type "AudioComponent Object Reference") (`New Volume Level` :type "Float (double-precision)"))
  (`AudioComponent.SetVolumeMultiplier` Song (* (`KismetMathLibrary.FMax` `New Volume Level` (`self.Minimum Volume Level`)) (`self.Master Volume Adjustment`))))

(fn `Is Adjustable?`
  (returns (Adjustable :type Boolean))
  ;[0.9 0.3 1] Are the songs adjustable right now? - KAB
  (return (and (`self.Is Playing`) (`self.Has Setup Songs`) (not (`self.Is Finished`)))))

(fn `Pause`
  ;[0.9 0.3 1] Pause all songs - KAB
  (bind _adjustable (`self.Is Adjustable?`))
  (if _adjustable
    (for _array_element _
      (`AudioComponent.SetPaused` _array_element true))
    (set `self.Is Playing` false)))

(fn `Register Tension`
  (params (Actor :type "Actor Object Reference"))
  (bind _returnvalue (`KismetSystemLibrary.GetObjectName` Actor))
  ;[0.9 0.3 1] Register new tension and, if changed, update audio using last progress - KAB
  (if (not (`BlueprintSetLibrary.Set_Contains` (`self.Tension Actors`) _returnvalue))
    (`BlueprintSetLibrary.Set_Add` (`self.Tension Actors`) _returnvalue)
    (`self.Update Progress` (`self.Last Progress`))))

(fn `Remove Song Handle`
  (params (`Song Handle` :type "AudioComponent Object Reference"))
  (bind _master_volume_adjustment (`self.Master Volume Adjustment`))
  ;[0.9 0.3 1] Fade out the song handle and then destroy it - KAB
  (`/Engine/EditorBlueprintResources/StandardMacros.IsValid` `Song Handle`
    (:`Is Valid`
      (`AudioComponent.FadeOut` `Song Handle` _master_volume_adjustment 0.0 "Linear")
      (`KismetSystemLibrary.K2_SetTimer` `Song Handle` "Destroy" _master_volume_adjustment) ; This destroys only if spawned with Autodestroy enabled
    )))

(fn `Resume`
  ;[0.9 0.3 1] Resume all songs - KAB
  (bind _adjustable (`self.Is Adjustable?`))
  (if _adjustable
    (for _array_element _
      (`AudioComponent.SetPaused` _array_element false))
    (set `self.Is Playing` true)))

(fn `Start Playing`
  (bind _song_handle_basket (`self.Song Handle Basket`))
  (bind _song_handle_basket_2 (`self.Song Handle Basket`))
  (bind _minimum_volume_level (`self.Minimum Volume Level`))
  ;[0.9 0.3 1] Clear existing song handles (if any), then allocate and start songs - KAB
  (bind _asbod_game_instance_bp (cast `/Game/Blueprints/BOD_GameInstanceBP` (`GameplayStatics.GetGameInstance`)))
  (set `self.Master Volume Adjustment` (`KismetMathLibrary.FMax` (`/Game/Blueprints/BOD_GameSettingsBP.MusicVolume` (`/Game/Blueprints/BOD_GameInstanceBP.Settings` _asbod_game_instance_bp)) (`self.Minimum Volume Level`)))
  (if (`self.Has Setup Songs`)
    (for _array_element _song_handle_basket
      (`self.Remove Song Handle` _array_element))
    (`KismetArrayLibrary.Array_Clear` _song_handle_basket))
  (`|ExecutionSequence`
    (:`then_0`
      (bind _returnvalue (`GameplayStatics.SpawnSound2D` (`self.Foundation Song`) (`self.Master Volume Adjustment`) 1.0 0.0 null false false))
      (bind _output_get (set `self.Foundation Song Handle` _returnvalue))
      (`KismetArrayLibrary.Array_Add` _song_handle_basket_2 _output_get))
    (:`then_1`
      (bind _returnvalue_2 (`GameplayStatics.SpawnSound2D` (`self.Progress 1 Song`) _minimum_volume_level 1.0 0.0 null false false))
      (bind _output_get_2 (set `self.Progress 1 Song Handle` _returnvalue_2))
      (`KismetArrayLibrary.Array_Add` _song_handle_basket_2 _output_get_2))
    (:`then_2`
      (bind _returnvalue_3 (`GameplayStatics.SpawnSound2D` (`self.Progress 2 Song`) _minimum_volume_level 1.0 0.0 null false false))
      (bind _output_get_3 (set `self.Progress 2 Song Handle` _returnvalue_3))
      (`KismetArrayLibrary.Array_Add` _song_handle_basket_2 _output_get_3))
    (:`then_3`
      (bind _returnvalue_4 (`GameplayStatics.SpawnSound2D` (`self.Boost Song`) _minimum_volume_level 1.0 0.0 null false false))
      (bind _output_get_4 (set `self.Boost Song Handle` _returnvalue_4))
      (`KismetArrayLibrary.Array_Add` _song_handle_basket_2 _output_get_4))
    (:`then_4`
      (bind _returnvalue_5 (`GameplayStatics.SpawnSound2D` (`self.Tension Song`) _minimum_volume_level 1.0 0.0 null false false))
      (bind _output_get_5 (set `self.Tension Song Handle` _returnvalue_5))
      (`KismetArrayLibrary.Array_Add` _song_handle_basket_2 _output_get_5))
    (:`then_5`
      (bind _returnvalue_6 (`GameplayStatics.SpawnSound2D` (`self.Finished Song`) _minimum_volume_level 1.0 0.0 null false false))
      (bind _output_get_6 (set `self.Finished Song Handle` _returnvalue_6))
      (`KismetArrayLibrary.Array_Add` _song_handle_basket_2 _output_get_6))
    (:`then_6`
      (set `self.Has Setup Songs` true)
      (set `self.Is Playing` true)
      (set `self.Is Finished` false))
    (:`then_7`
      (`self.Update Progress` 0.0))))

(fn `Unregister Tension`
  (params (Actor :type "Actor Object Reference"))
  (bind _returnvalue (`KismetSystemLibrary.GetObjectName` Actor))
  (bind _tension_actors (`self.Tension Actors`))
  ;[0.9 0.3 1] Unregister tension and, if changed, update audio using last progress - KAB
  (if (`BlueprintSetLibrary.Set_Contains` _tension_actors _returnvalue)
    (`BlueprintSetLibrary.Set_Remove` _tension_actors _returnvalue)
    (`self.Update Progress` (`self.Last Progress`))))

(fn `Update Progress`
  (params (Progress :type "Float (double-precision)"))
  (locals (`New Tension Enabled` :type Boolean))
  (bind _tension_song_handle (`self.Tension Song Handle`))
  (bind (_returnvalue_x _returnvalue_y _returnvalue_z) (`KismetMathLibrary.BreakVector` (`CurveVector.GetVectorValue` (`self.Volume Curves`) Progress)))
  ;[0.9 0.3 1] The core driver for the dynamic music: a 0..1 "progress" value that changes volumes of musical layers - KAB
  (bind _adjustable (`self.Is Adjustable?`))
  (set `self.Last Progress` Progress)
  (if _adjustable
    (`|ExecutionSequence`
      (:`then_0`
        (`self.Faded Adjustment` (`self.Foundation Song Handle`) _returnvalue_x))
      (:`then_1`
        (`self.Faded Adjustment` (`self.Progress 1 Song Handle`) _returnvalue_y))
      (:`then_2`
        (`self.Faded Adjustment` (`self.Progress 2 Song Handle`) _returnvalue_z))
      (:`then_3`
        (bind _output_get (set `local.New Tension Enabled` (> (`BlueprintSetLibrary.Set_Length` (`self.Tension Actors`)) 0)))
        (if (!= _output_get (`self.Tension Enabled`))
          (set `self.Tension Enabled` _output_get)
          (if _output_get
            (`self.Faded Adjustment` _tension_song_handle 1.0)
            (else
              (`self.Faded Adjustment` _tension_song_handle))))))))

(fn `UserConstructionScript`)